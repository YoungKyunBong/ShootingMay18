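; Player hero character for a top-down style shooter, moving along world axes with a visible mouse cursor.
; BeginPlay spawns a gun on the mesh's GunSocket and a MousePointBP marker, which moves to the cursor hit on each left press or release.
; Holding left click fires the gun and enables collision on hand components attached to hand bones for punching.
; DecreaseHP tracks damage, destroying hero and gun and restarting the level at zero health.
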(event EventBeginPlay
  (Variables|Default|SetHP 1e+02)
  (bind _asshooter_game_mode (Utilities|Casting|CastToShooterGameMode (Game|GetGameMode)))
  (Variables|Default|SetGameMode _asshooter_game_mode)
  (bind _returnvalue (Game|SpawnActorfromClass "/Game/UI/MousePointBP.MousePointBP_C" (Math|Conversions|ToTransform(Vector) (Transformation|GetActorLocation)) "Undefined" 0 0))
  (Variables|Default|SetMouseClickPoint _returnvalue)
  (Variables|/Script/Engine.PlayerController|SetbShowMouseCursor (Game|GetPlayerController 0) true)
  (Variables|/Script/Engine.CharacterMovementComponent|SetbOrientRotationToMovement (Variables|Character|GetCharacterMovement) false)
  (bind _returnvalue_2 (Game|SpawnActorfromClass "/Game/GunBP.GunBP_C" (Transformation|GetWorldTransform (Variables|Character|GetMesh)) "Undefined" 0 0))
  (bind _output_get (Variables|Default|SetGun _returnvalue_2))
  (Transformation|AttachComponentToComponent _output_get (Variables|Character|GetMesh) "GunSocket" "SnapToTarget" "SnapToTarget" "KeepWorld" true))

(event EventDecreaseHP
  (params (amount :type Float%20%28single-precision%29))
  (bind _output_get (Variables|Default|SetHP (- (Variables|Default|GetHP) amount)))
  (if (<= _output_get 0.0)
    (Input|DisableInput 0)
    (Actor|DestroyActor self)
    (Development|ExecuteConsoleCommand "restartlevel")))

(event Input|ActionEvents|InputActionLeftMouseClicked
  (params (Key :type Key%20Structure :default "AnyKey"))
  (bind _gun (Variables|Default|GetGun))
  (bind _righthand (Variables|Default|GetRightHand))
  (:Pressed
    (Default|StartFiring _gun)
    (Variables|Default|SetIs%20Punching true)
    (Collision|SetCollisionEnabled _righthand "QueryAndPhysics")
    (Transformation|SetActorLocation (Variables|Default|GetMouseClickPoint) (.Location (Collision|BreakHitResult (.HitResult (Game|Player|GetHitResultUnderCursorbyChannel (Game|GetPlayerController 0) "TraceTypeQuery1" true)))) false false :!label _label))
  (:Released
    (Default|StopFiring _gun)
    (Variables|Default|SetIs%20Punching false)
    (Collision|SetCollisionEnabled _righthand "NoCollision")
    (goto _label)))

(event Input|AxisEvents|InputAxisMoveForeward
  (params (AxisValue :type Float%20%28single-precision%29))
  (Pawn|Input|AddMovementInput "1.000000, 0, 0" AxisValue false))

(event Input|AxisEvents|InputAxisMoveRight
  (params (AxisValue :type Float%20%28single-precision%29))
  (Pawn|Input|AddMovementInput "0,1.000000, 0" AxisValue false))

(fn ConstructionScript
  (bind _mesh (Variables|Character|GetMesh))
  (Transformation|AttachComponentToComponent (Variables|Default|GetRightHand) _mesh "hand_r" "KeepRelative" "KeepRelative" "KeepRelative" true)
  (Transformation|AttachComponentToComponent (Variables|Default|GetLeftHand) _mesh "hand_l" "KeepRelative" "KeepRelative" "KeepRelative" true))