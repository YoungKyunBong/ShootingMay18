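; EnemyBP is an enemy actor that damages the hero on contact and dies when its own HP runs out.
; It starts with 100 HP, and its DecreaseHP event subtracts damage and destroys the actor at zero.
; Overlapping a HeroBP hits it immediately, then a looping one-second timer repeats HeroDamage through the hero's DecreaseHP until the overlap ends.
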(event Custom|HeroDamage
  (Default|DecreaseHP (stale Collision|EventActorBeginOverlap _ashero_bp) 2e+01))

(event EventBeginPlay
  (Variables|Default|SetHP 1e+02))

(event Collision|EventActorBeginOverlap
  (params (OtherActor :type Actor%20Object%20Reference))
  (bind _ashero_bp (Utilities|Casting|CastToHeroBP OtherActor))
  (CallFunction|HeroDamage)
  (Utilities|Time|SetTimerbyFunctionName 0 "HeroDamage" 1.0 true))

(event EventTick
  (params (DeltaSeconds :type Float%20%28single-precision%29)))

(event Collision|EventActorEndOverlap
  (params (OtherActor :type Actor%20Object%20Reference))
  (Utilities|Casting|CastToHeroBP OtherActor)
  (Utilities|Time|ClearTimerbyFunctionName 0 "HeroDamage"))

(event EventDecreaseHP
  (params (Amount :type Float%20%28single-precision%29))
  (bind _output_get (Variables|Default|SetHP (- (Variables|Default|GetHP) Amount)))
  (if (<= _output_get 0.0)
    (Actor|DestroyActor)))

(fn ConstructionScript)