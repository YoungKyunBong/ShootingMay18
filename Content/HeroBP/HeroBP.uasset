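; HeroBP is the player character, with world-axis movement, yaw turning, a spawned gun and health.
; On BeginPlay it sets HP, spawns a GunBP and attaches its mesh to the GunSocket on the character mesh.
; The TriggerBullet input starts and stops the gun's fire.
; DecreaseHP prints remaining health and, at zero or below, hides the capsule and its children, then restarts the level after a short delay.
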(event EventBeginPlay
  (Variables|Default|SetHP 1e+02)
  (bind _returnvalue (Game|SpawnActorfromClass "/Game/Gun/GunBP.GunBP_C" (Transformation|GetWorldTransform (Variables|Character|GetMesh)) "Undefined" 0 0))
  (bind _output_get (Variables|Default|SetGun _returnvalue))
  (Transformation|AttachComponentToComponent (Variables|/Game/Gun/GunBP.GunBP_C|GetSK_FPGun _output_get) (Variables|Character|GetMesh) "GunSocket" "SnapToTarget" "SnapToTarget" "KeepWorld" true))

(event Collision|EventActorBeginOverlap
  (params (OtherActor :type Actor%20Object%20Reference)))

(event EventDecreaseHP
  (params (Amount :type Float%20%28single-precision%29))
  (bind _output_get (Variables|Default|SetHP (- (Variables|Default|GetHP) Amount)))
  (Development|PrintString (Utilities|String|ToString(Float) _output_get) true true "(R=0.000000,G=0.660000,B=1.000000,A=1.000000)" 1.0)
  (if (<= _output_get 0.0)
    (Rendering|SetVisibility (Variables|Collision|GetCapsuleComponent) false true)
    (Utilities|FlowControl|Delay 0.1)
    (Development|ExecuteConsoleCommand "RestartLevel")))

(event EventTick
  (params (DeltaSeconds :type Float%20%28single-precision%29)))

(event Input|ActionEvents|InputActionTriggerBullet
  (params (Key :type Key%20Structure :default "AnyKey"))
  (bind _gun (Variables|Default|GetGun))
  (:Pressed
    (Default|StartFire _gun))
  (:Released
    (Default|StopFire _gun)))

(event Input|AxisEvents|InputAxisMoveForward
  (params (AxisValue :type Float%20%28single-precision%29))
  (Pawn|Input|AddMovementInput "10.000000, 0, 0" AxisValue false))

(event Input|AxisEvents|InputAxisMoveRight
  (params (AxisValue :type Float%20%28single-precision%29))
  (Pawn|Input|AddMovementInput "0.000000,10.000000, 0" AxisValue false))

(event Input|AxisEvents|InputAxisTurnRight
  (params (AxisValue :type Float%20%28single-precision%29))
  (Transformation|AddActorLocalRotation (Math|Rotator|MakeRotator 0.0 0.0 (* AxisValue 3.0)) false false))

(fn ConstructionScript)