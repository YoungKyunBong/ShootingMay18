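; My_HeroBP is the player hero, which moves, turns, shoots and tracks its health.
; On BeginPlay it caches My_GamoMode, sets HP and spawns a My_GunBP snapped to the mesh's GunPoint socket.
; Input drives movement along fixed world axes and yaw rotation, while the Shout action starts and stops gun fire.
; DownHP subtracts damage, updates the game mode's UI health bar and restarts the level at zero HP via console command.
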(event EventBeginPlay
  (bind _asmy_gamo_mode (Utilities|Casting|CastToMy_GamoMode (Game|GetGameMode)))
  (Variables|Default|SetMyGameMode _asmy_gamo_mode)
  (Variables|Default|SetHP 1e+02)
  (bind _returnvalue (Game|SpawnActorfromClass "/Game/Gun/My_GunBP.My_GunBP_C" (Transformation|GetWorldTransform (Variables|Character|GetMesh)) "Undefined" 0 0))
  (bind _output_get (Variables|Default|SetGun _returnvalue))
  (Transformation|AttachComponentToComponent _output_get (Variables|Character|GetMesh) "GunPoint" "SnapToTarget" "SnapToTarget" "KeepRelative" true))

(event Collision|EventActorBeginOverlap
  (params (OtherActor :type Actor%20Object%20Reference)))

(event EventDownHP
  (params (DisHP :type Float%20%28single-precision%29))
  (bind _output_get (Variables|Default|SetHP (- (Variables|Default|GetHP) DisHP)))
  (Default|SetHPBar (Variables|/Game/My_GamoMode.My_GamoMode_C|GetMyUI (Variables|Default|GetMyGameMode)) _output_get)
  (if (<= _output_get 0.0)
    (Development|ExecuteConsoleCommand "RestartLevel")))

(event EventTick
  (params (DeltaSeconds :type Float%20%28single-precision%29)))

(event Input|ActionEvents|InputActionShout
  (params (Key :type Key%20Structure :default "AnyKey"))
  (bind _gun (Variables|Default|GetGun))
  (:Pressed
    (Default|StartFire _gun))
  (:Released
    (Default|EndFire _gun)))

(event Input|AxisEvents|InputAxisMove_FB
  (params (AxisValue :type Float%20%28single-precision%29))
  (Pawn|Input|AddMovementInput "1.000000, 0, 0" AxisValue false))

(event Input|AxisEvents|InputAxisMove_LR
  (params (AxisValue :type Float%20%28single-precision%29))
  (Pawn|Input|AddMovementInput "0,1.000000, 0" AxisValue false))

(event Input|AxisEvents|InputAxisTurn
  (params (AxisValue :type Float%20%28single-precision%29))
  (Transformation|AddActorLocalRotation (Math|Rotator|MakeRotator 0.0 0.0 (* AxisValue 3.0)) false false))

(fn ConstructionScript)